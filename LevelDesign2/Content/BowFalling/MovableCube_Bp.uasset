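; MovableCube_Bp is a cube that the side-scroller character can push while the game instance flags the player as small.
; Overlapping the YAxisCollison volume while small turns on physics simulation for the cube and sets the character's IsPushing flag.
; When the character leaves the volume, physics simulation is switched off and IsPushing is cleared, whatever the player's size.
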(event `self.Y Axis Collison.OnComponentBeginOverlap`
  (params (OverlappedComponent :type "PrimitiveComponent Object Reference") (OtherActor :type "Actor Object Reference") (OtherComp :type "PrimitiveComponent Object Reference") (OtherBodyIndex :type Integer) (bFromSweep :type Boolean) (SweepResult :type "HitResult Structure (by ref)"))
  (bind _asside_scroller_character (cast `/Game/SideScrollerBP/Blueprints/SideScrollerCharacter` OtherActor))
  (bind _asbp_game_instance (cast `/Game/SideScrollerBP/Blueprints/BP_GameInstance` (`GameplayStatics.GetGameInstance`)))
  (if (`/Game/SideScrollerBP/Blueprints/BP_GameInstance.Is the player small?` _asbp_game_instance)
    (`PrimitiveComponent.SetSimulatePhysics` (`self.Cube`) true)
    (set `/Game/SideScrollerBP/Blueprints/SideScrollerCharacter.IsPushing` true _asside_scroller_character)))

(event `self.Y Axis Collison.OnComponentEndOverlap`
  (params (OverlappedComponent :type "PrimitiveComponent Object Reference") (OtherActor :type "Actor Object Reference") (OtherComp :type "PrimitiveComponent Object Reference") (OtherBodyIndex :type Integer))
  (bind _asside_scroller_character (cast `/Game/SideScrollerBP/Blueprints/SideScrollerCharacter` OtherActor))
  (`PrimitiveComponent.SetSimulatePhysics` (`self.Cube`) false)
  (set `/Game/SideScrollerBP/Blueprints/SideScrollerCharacter.IsPushing` false _asside_scroller_character))

(fn `UserConstructionScript`)